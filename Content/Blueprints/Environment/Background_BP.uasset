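; Background actor that scrolls horizontally with the camera to create a parallax effect.
; On BeginPlay it caches the player camera manager, its starting location and the actor's own start position.
; Each tick it offsets its X by the camera's X travel scaled by MoveAmount, keeping Y and Z fixed.
; An automatic vertical scroll-and-wrap routine remains in the graph but never runs.
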(event EventBeginPlay
  (bind _output_get (Variables|Default|Setcamera (Variables|/Script/Engine.PlayerController|GetPlayerCameraManager (Game|GetPlayerController 0))))
  (Variables|Default|SetstartCameraPos (Camera|GetCameraLocation _output_get))
  (Variables|Default|SetstartPos (Transformation|GetActorLocation)))

(event Collision|EventActorBeginOverlap
  (params (OtherActor :type Actor%20Object%20Reference)))

(event EventTick
  (params (DeltaSeconds :type Float%20%28single-precision%29))
  (bind _startpos (Variables|Default|GetstartPos))
  (Transformation|SetActorLocation (Math|Vector|MakeVector (+ (.x _startpos) (* (Variables|Default|GetMove%20Amount) (- (.x (Camera|GetCameraLocation (Variables|Default|Getcamera))) (.x (Variables|Default|GetstartCameraPos))))) (.y _startpos) (.z _startpos)) false false))

(fn ConstructionScript)