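; QueenGambitGameMode is a game mode that completes the level once every pumpkin collectable has been collected.
; On BeginPlay it switches the player's view to the level's DefaultCamera, gathers pumpkin-type Collectables and binds to each one's collected event.
; Each collection removes that pumpkin from the tracked array, and an empty array opens the LevelComplete level.
; A separate AddScore function accumulates the score.
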(event Custom|GetAllPumpkin
  ;[1 1 1] Get All pumpkin in Level
  (bind _outactors (Actor|GetAllActorsOfClass "/Game/Blueprints/Interactables/Collectable.Collectable_C"))
  (for _array_element _outactors
    (if (Utilities|Enum|Equal(Enum) (Variables|/Game/Blueprints/Interactables/Collectable.Collectable_C|GetCollectableType _array_element) "NewEnumerator0")
      (Utilities|Array|AddUnique (Variables|Default|GetPumpkins) _array_element)))
  (Variables|Default|SetPumpkinAmount (Utilities|Array|Length (Variables|Default|GetPumpkins))))

(event Custom|RemovePumpkin
  (params (collectable :type Collectable%20Object%20Reference))
  (bind _pumpkins (Variables|Default|GetPumpkins))
  ;[1 1 1] Assign Pumpin Event
  (Utilities|Array|RemoveItem _pumpkins collectable)
  (if (== (Utilities|Array|Length _pumpkins) 0)
    (CallFunction|LevelComplected)))

(event Custom|LevelComplected
  (Game|OpenLevel(byName) "LevelComplete"))

(event Custom|AssignPumpinEvent
  ;[1 1 1] Assign Pumpin Event
  (for _array_element (Variables|Default|GetPumpkins)
    (EventDispatchers|BindEventtoOnPumpkinCollected _array_element (delegate Custom|RemovePumpkin))))

(event Custom|Set%20Camera
  ;[1 1 1] Set Camera
  (bind _outactors (Actor|GetAllActorsOfClass "/Game/Blueprints/Gameplay/DefaultCamera.DefaultCamera_C"))
  (Game|Player|SetViewTargetwithBlend (Game|GetPlayerController 0) (Utilities|Array|Get(acopy) _outactors) 0.0 "VTBlend_Linear" 0.0 false))

(event EventBeginPlay
  (CallFunction|SetCamera)
  (CallFunction|GetAllPumpkin)
  (CallFunction|AssignPumpinEvent))

(event EventTick
  (params (DeltaSeconds :type Float%20%28single-precision%29)))

(fn ConstructionScript)

(fn AddScore
  (params (Amount :type Integer))
  (Variables|Default|SetScore (+ Amount (Variables|Default|GetScore))))