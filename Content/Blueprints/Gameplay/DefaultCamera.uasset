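; Default side-view camera actor that follows the player's Queen character.
; On BeginPlay it casts the player character to Queen and stores it.
; Each Tick, while that reference is valid, it moves its root to the player's X and Z minus a camera offset, keeping its own Y as the base so it tracks in a plane without sweeping.
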(event EventBeginPlay
  (bind _asqueen (Utilities|Casting|CastToQueen (Game|GetPlayerCharacter 0)))
  (Variables|Default|SetPlayer _asqueen))

(event Collision|EventActorBeginOverlap
  (params (OtherActor :type Actor%20Object%20Reference)))

(event EventTick
  (params (DeltaSeconds :type Float%20%28single-precision%29))
  (bind _player (Variables|Default|GetPlayer))
  (bind _rootcomponent (Variables|/Script/Engine.Actor|GetRootComponent _player))
  (bind _returnvalue (Transformation|GetWorldLocation _rootcomponent))
  (if (Utilities|IsValid (Variables|Default|GetPlayer))
    (Transformation|SetWorldLocation (Variables|Default|GetDefaultSceneRoot) (- (Math|Vector|MakeVector (.x _returnvalue) (.y (Transformation|GetWorldLocation (Variables|Default|GetDefaultSceneRoot))) (.z _returnvalue)) (Variables|Default|GetCamera%20Offset)) false false)))

(fn ConstructionScript)