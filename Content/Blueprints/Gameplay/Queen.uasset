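; Queen is the side-scrolling, flipbook-animated player character that runs, jumps, climbs ladders and attacks with a sword.
; Input drives movement, turning via controller yaw and switching flipbooks.
; Tick runs two ladder overlap spheres that limit upward climbing and restore Walking from Flying, draws debug spheres, and triggers sphere-overlap damage on attack frame 5.
; A HealthSystem handles incoming damage, opening GameOver at zero, and BeginPlay adds the game UI.
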(event Custom|Rotate%20Sprite
  (bind _returnvalue (Pawn|GetController))
  ;[1 1 1] Rotate Sprite
  (if (Variables|Movement|GetIsMovingRight)
    (Pawn|SetControlRotation _returnvalue (Math|Rotator|MakeRotator 0.0 0.0 0.0))
    (else
      (Pawn|SetControlRotation _returnvalue (Math|Rotator|MakeRotator 0.0 0.0 1.8e+02)))))

(event Custom|CheckClimbing
  ;[1 1 1] Ladder detection
  (CallFunction|CheckLadderContact)
  (CallFunction|CheckLaddderinRange))

(event Custom|CheckLaddderInRange
  (bind _returnvalue (Transformation|GetActorLocation))
  (bind _returnvalue_2 (Math|Vector|MakeVector 0.0 0.0 1.2e+02))
  (bind _laddetdetectorrange (Variables|Climbing|GetladdetDetectorRange))
  (bind _returnvalue_3 (+ _returnvalue _returnvalue_2))
  ;[1 1 1] Check if Ladder is in range
  (Rendering|Debug|DrawDebugSphere _returnvalue_3 _laddetdetectorrange 12 "(R=0.000000,G=1.000000,B=0.016063,A=1.000000)" 0.0)
  (bind _returnvalue_4 (Collision|SphereOverlapActors _returnvalue_3 _laddetdetectorrange (Utilities|Array|MakeArray "ObjectTypeQuery1") "/Game/Blueprints/Interactables/Ladder.Ladder_C"))
  (if _returnvalue_4
    (Variables|Climbing|SetcanClimb true)
    (else
      (Variables|Climbing|SetcanClimb false))))

(event Custom|Climbing%20Mode
  ;[1 1 1] Enter Climbing mode
  (if (Math|Boolean|NANDBoolean (Variables|Climbing|GetladderDetected) (Variables|Climbing|GetisClimbing))
    (Variables|Climbing|SetisClimbing true)
    (Pawn|Components|CharacterMovement|SetMovementMode (Variables|Character|GetCharacterMovement) "MOVE_Flying" 0)))

(event Custom|Exit%20Climbing%20Mode
  ;[1 1 1] Exit Climbing
  (if (Variables|Climbing|GetisClimbing)
    (if (not (Variables|Climbing|GetladderDetected))
      (Variables|Climbing|SetisClimbing false)
      (Pawn|Components|CharacterMovement|SetMovementMode (Variables|Character|GetCharacterMovement) "MOVE_Walking" 0))))

(event Custom|Climbing
  (bind _returnvalue (Input|AxisValues|GetVerticalMovement))
  ;[1 1 1] Climbing
  (Pawn|Input|AddMovementInput "0.000000,0.000000,1.000000" (Math|Float|SelectFloat (* (Variables|Climbing|GetclimbSpeed) _returnvalue) (* (Math|Float|Clamp(Float) _returnvalue -1.0 0.0) (Variables|Climbing|GetclimbSpeed)) (Variables|Climbing|GetcanClimb)) false))

(event Custom|Climbing%20Animation
  ;[1 1 1] Climbing Animation
  (if (Variables|Climbing|GetisClimbing)
    (Sprite|SetFlipbook (Variables|Default|GetSprite) (select (> (Math|Float|Absolute(Float) (Input|AxisValues|GetVerticalMovement)) 0.0) (Variables|Animation|GetLadder-Climbing_Animation) (Variables|Animation|GetLadder-Idle_Animation)))))

(event Custom|Damage%20Debug
  ;[1 1 1] Damage Debug
  (bind _attackposition (CallFunction|AttackPosition))
  (Rendering|Debug|DrawDebugSphere _attackposition (Variables|Attacking|GetattackRadius) 12 "(R=1.000000,G=0.000000,B=0.402194,A=1.000000)" 0.0))

(event Custom|Play%20Movement%20Animation
  (bind _returnvalue (Pawn|GetMovementComponent))
  (bind _velocity (Variables|/Script/Engine.MovementComponent|GetVelocity _returnvalue))
  ;[1 1 1] Movement Animation : Check if player is on the ground then toggle between Idle and Run animation
  (if (Pawn|Components|CharacterMovement|IsWalking (Variables|Character|GetCharacterMovement))
    (if (not (Variables|Attacking|GetisAttacking))
      (if (== (.z _velocity) 0.0)
        (Sprite|SetFlipbook (Variables|Default|GetSprite) (select (== (.x _velocity) 0.0) (Variables|Animation|GetIdle_Animation) (Variables|Animation|GetRun_Animation)))))))

(event Custom|Deal%20Damage
  ;[1 1 1] Deal Damage
  (bind _returnvalue (Actor|GetActorOfClass "Queen_C"))
  (bind _attackposition (CallFunction|AttackPosition))
  (bind (_outactors _returnvalue_2) (Collision|SphereOverlapActors _attackposition (Variables|Attacking|GetattackRadius) (Utilities|Array|MakeArray "ObjectTypeQuery7") 0 (Utilities|Array|MakeArray _returnvalue)))
  (if _returnvalue_2
    (for _array_element _outactors
      (Class|BPIDamageable|TakeDamage(Message) _array_element (Variables|Attacking|GetDamageAmount)))))

(event Custom|Attack%20Event
  ;[1 1 1] Attack Animation Event
  (if (Variables|Attacking|GetisAttacking)
    (if (Variables|Attacking|GetcanDamage)
      (if (== (Class|PaperFlipbookComponent|GetPlaybackPositioninFrames (Variables|Default|GetSprite)) 5)
        (Variables|Attacking|SetcanDamage false)
        (CallFunction|DealDamage)))))

(event Custom|Display%20UI
  ;[1 1 1] Displaying Game UI on Screen
  (bind _returnvalue (UserInterface|CreateWidget "/Game/Blueprints/UI/Game_UI.Game_UI_C"))
  (bind _output_get (Variables|Health|SetUI _returnvalue))
  (UserInterface|Viewport|AddtoViewport _output_get 0))

(event Custom|Flip%20Sprite
  ;[1 1 1] Flipping Sprite. Not Working
  (if (Variables|Movement|GetIsMovingRight)
    (Transformation|SetActorScale3D "1.000000,1.000000,1.000000")
    (else
      (Transformation|SetActorScale3D "-1.000000,1.000000,1.000000"))))

(event Custom|CheckLadderContact
  (bind _returnvalue (Transformation|GetActorLocation))
  (bind _laddetdetectorrange (Variables|Climbing|GetladdetDetectorRange))
  ;[1 1 1] Check if ladderr in contact
  (Rendering|Debug|DrawDebugSphere _returnvalue _laddetdetectorrange 12 "(R=1.000000,G=0.839822,B=0.000000,A=1.000000)" 0.0)
  (bind _returnvalue_2 (Collision|SphereOverlapActors _returnvalue _laddetdetectorrange (Utilities|Array|MakeArray "ObjectTypeQuery1") "/Game/Blueprints/Interactables/Ladder.Ladder_C"))
  (if _returnvalue_2
    (Variables|Climbing|SetladderDetected true)
    (else
      (Variables|Climbing|SetladderDetected false)
      (Variables|Climbing|SetcanClimb false)
      (CallFunction|ExitClimbingMode))))

(event EventBeginPlay
  ;[1 1 1] Event BeginePlay
  (Default|SetUp (Variables|Default|GetHealthSystem) (Variables|Health|GetHealth))
  (CallFunction|DisplayUI))

(event EventTakeDamage
  (params (amount :type Integer))
  ;[1 1 1] Recieving Damage
  (bind _currenthealth (Default|TakeDamage (Variables|Default|GetHealthSystem) amount))
  (Components|Activation|Activate (Variables|Default|GetParticleSystem_Blood) false)
  (if (<= _currenthealth 0)
    (Game|OpenLevel(byName) "GameOver")))

(event EventTick
  (params (DeltaSeconds :type Float%20%28single-precision%29))
  ;[1 1 1] Event Tick
  (CallFunction|PlayMovementAnimation)
  (CallFunction|CheckClimbing)
  (CallFunction|AttackEvent)
  (CallFunction|DamageDebug))

(event Input|ActionEvents|InputActionAttack
  (params (Key :type Key%20Structure :default "None"))
  ;[1 1 1] Attacking
  (:Pressed
    (if (not (Variables|Attacking|GetisAttacking))
      (Audio|PlaySound2D "/Game/Audio/sword_sound.sword_sound" 0.2 1.0 0.0 0 0)
      (Variables|Attacking|SetisAttacking true)
      (Sprite|SetFlipbook (Variables|Default|GetSprite) (Variables|Animation|GetAttack_Animation))
      (Variables|Movement|Setspeed 0.2)
      (Utilities|FlowControl|Delay (Variables|Attacking|GetAttackDelay))
      (Variables|Attacking|SetisAttacking false)
      (Variables|Attacking|SetcanDamage true)
      (Variables|Movement|Setspeed 1.0))))

(event Input|ActionEvents|InputActionJump
  (params (Key :type Key%20Structure :default "None"))
  ;[1 1 1] Movement Animation : Check if player is on the ground then toggle between Idle and Run animation
  ;;[1 1 1] Jump Animation
  (:Pressed
    (Sprite|SetFlipbook (Variables|Default|GetSprite) (Variables|Animation|GetJump_Animation))))

(event Input|ActionEvents|InputActionJump
  (params (Key :type Key%20Structure :default "None"))
  ;[1 1 1] Jumping
  (:Pressed
    (Character|Jump)
    (Audio|PlaySound2D "/Game/Audio/sfx_jump.sfx_jump" 0.2 1.0 0.0 0 0))
  (:Released
    (Character|StopJumping)))

(event Input|AxisEvents|InputAxisVerticalMovement
  (params (AxisValue :type Float%20%28single-precision%29))
  (CallFunction|ClimbingAnimation)
  (if (and (> (Math|Float|Absolute(Float) AxisValue) 0.0) (Variables|Climbing|GetladderDetected))
    (CallFunction|ClimbingMode)
    (CallFunction|ClimbING)))

(event Input|AxisEvents|InputAxisHorizontalMovement
  (params (AxisValue :type Float%20%28single-precision%29))
  ;[1 1 1] Movement
  (Math|Float|CompareFloat AxisValue 0.0
    (:>
      (Variables|Movement|SetIsMovingRight true))
    (:<
      (Variables|Movement|SetIsMovingRight false)))
  (CallFunction|RotateSprite)
  (Pawn|Input|AddMovementInput (* (Class|KismetMathLibrary|VectorForward) (Variables|Movement|Getspeed)) (Input|AxisValues|GetHorizontalMovement) false))

(fn ConstructionScript)

(fn AttackPosition
  ;[1 1 1] Check where the player is facing and add the apporotite offset
  (return (+ (Math|Vector|MakeVector (Math|Float|SelectFloat (Variables|Attacking|GetAttackXOffset) (* (Variables|Attacking|GetAttackXOffset) -1.0) (Variables|Movement|GetIsMovingRight)) 0.0 0.0) (Transformation|GetActorLocation))))