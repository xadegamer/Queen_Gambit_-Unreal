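; Base 2D flipbook enemy that patrols waypoints, chases and attacks the player in range, and awards score on death.
; A Tick-driven Patrol/Chase state machine switches on distance checks, moving via MoveComponentTo timed by distance over speed, with optional vertical following when flying.
; Attacks deal sphere-overlap damage on a chosen animation frame.
; HealthSystem feeds a health bar shown while the Queen overlaps its view collider; debug spheres show waypoints and damage area.
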(event OnComponentBeginOverlap(Health_ViewCollider)
  (params (OverlappedComponent :type Primitive%20Component%20Object%20Reference) (OtherActor :type Actor%20Object%20Reference) (OtherComp :type Primitive%20Component%20Object%20Reference) (OtherBodyIndex :type Integer) (bFromSweep :type Boolean) (SweepResult :type Hit%20Result%20Structure%20%28by%20ref%29))
  ;[1 1 1] Toggling health UI
  (Utilities|Casting|CastToQueen OtherActor)
  (Rendering|SetVisibility (Variables|Default|GetWidget) true false))

(event OnComponentEndOverlap(Health_ViewCollider)
  (params (OverlappedComponent :type Primitive%20Component%20Object%20Reference) (OtherActor :type Actor%20Object%20Reference) (OtherComp :type Primitive%20Component%20Object%20Reference) (OtherBodyIndex :type Integer))
  ;[1 1 1] Toggling health UI
  (Utilities|Casting|CastToQueen OtherActor)
  (Rendering|SetVisibility (Variables|Default|GetWidget) false false))

(event Custom|RewardPlayer
  ;[1 1 1] Reward Player
  (bind _asqueen_gambit_game_mode (Utilities|Casting|CastToQueenGambitGameMode (Game|GetGameMode)))
  (Default|AddScore _asqueen_gambit_game_mode (Variables|Properties|GetscoreAmount)))

(event Custom|Patrol
  (bind _waypoints (Variables|AI|GetWayPoints))
  (bind _currentwaypoint (Variables|AI|GetcurrentWayPoint))
  (bind _output (Utilities|Array|Get(acopy) _waypoints _currentwaypoint))
  ;[1 1 1] Moving to position - Since Speed = Distance / Time, Time = Distance / Speed.
  (CallFunction|ChangeAnimation (Variables|Animation|GetWalk%20Animation))
  (CallFunction|LookatPosition _output)
  (Components|MoveComponentTo (Variables|Default|GetDefaultSceneRoot1) _output "0, 0, 0" false false (/ (Math|Vector|VectorLength (- _output (Transformation|GetActorLocation))) (Variables|Properties|GetmoveSpeed)) false)
  (if (Utilities|Enum|Equal(Enum) (Variables|AI|GetAI%20State) "NewEnumerator0")
    (CallFunction|MovetoPosition)))

(event Custom|Death
  ;[1 1 1] Enemy Death
  (CallFunction|ChangeAnimation (Variables|Animation|GetDead%20Animation))
  (CallFunction|RewardPlayer)
  (Audio|PlaySound2D "/Game/Audio/DM-CGS-11.DM-CGS-11" 0.2 1.0 0.0 0 0)
  (Utilities|FlowControl|Delay 0.7)
  (Actor|DestroyActor))

(event Custom|AI%20State%20Machine
  (params (newState :type AI_State%20Enum :default "NewEnumerator0"))
  ;[1 1 1] AI State Machine
  (if (Utilities|Enum|NotEqual(Enum) newState (Variables|AI|GetAI%20State))
    (bind _output_get (Variables|AI|SetAI%20State newState))
    (switch Utilities|FlowControl|Switch|SwitchonAI_State _output_get
      (:NewEnumerator0
        (CallFunction|Patrol))
      (:NewEnumerator2
        _))
    (CallFunction|ChangeAnimation (Variables|Animation|GetWalk%20Animation))))

(event Custom|Attack
  ;[1 1 1] Attacking
  (Variables|Attacking|Setcan%20Damage true)
  (CallFunction|ChangeAnimation (Variables|Animation|GetIdle%20Animation))
  (Utilities|FlowControl|Delay (Variables|Attacking|Getattack%20Rate))
  (if (not (Variables|Properties|GetisDead))
    (CallFunction|ChangeAnimation (Variables|Animation|GetAttack%20Animation))
    (Utilities|FlowControl|Delay (Variables|Attacking|Getattack%20Duration))
    (if (Variables|AI|GetplayerInAttackRange)
      (CallFunction|Attack))))

(event Custom|Attack%20Event
  (bind _skeleton (Variables|Default|GetSkeleton))
  ;[1 1 1] Attack Event
  (if (Variables|Attacking|Getcan%20Damage)
    (if (and (== (Class|PaperFlipbookComponent|GetFlipbook _skeleton) (Variables|Animation|GetAttack%20Animation)) (== (Class|PaperFlipbookComponent|GetPlaybackPositioninFrames _skeleton) (Variables|Attacking|GetAttackEventFrame)))
      (Variables|Attacking|Setcan%20Damage false)
      (CallFunction|DealDamage))))

(event Custom|AI%20State%20Machine%20Tick
  ;[1 1 1] AI State Machine Tick
  (switch Utilities|FlowControl|Switch|SwitchonAI_State (Variables|AI|GetAI%20State)
    (:NewEnumerator0
      (CallFunction|ScanPlayer))
    (:NewEnumerator2
      (CallFunction|PatrolStateCondition))))

(event Custom|Stop%20Chasing%20Player
  (bind _returnvalue (Transformation|GetActorLocation))
  (bind _returnvalue_2 (Game|GetPlayerCharacter 0))
  (bind _isflying (Variables|AI|GetisFlying))
  (bind _returnvalue_3 (Transformation|GetActorLocation _returnvalue_2))
  (bind _returnvalue_4 (Math|Float|SelectFloat (.z _returnvalue_3) (.z _returnvalue) _isflying))
  (bind _returnvalue_5 (Math|Vector|MakeVector (.x _returnvalue_3) (.y _returnvalue) _returnvalue_4))
  ;[1 1 1] Chase Player
  (Components|MoveComponentTo (Variables|Default|GetDefaultSceneRoot1) _returnvalue_5 "0, 0, 0" false false (/ (Math|Vector|VectorLength (- _returnvalue_5 (Transformation|GetActorLocation))) (Variables|Properties|GetrunSpeed)) false) ; enters at Stop
)

(event Custom|Patrol%20State%20Condition
  ;[1 1 1] Attack if player in attack range amd go back to patrol if player is far
  (bind _in_range (CallFunction|PlayerinRange (Variables|AI|GetattackRange)))
  (if _in_range
    (Variables|AI|SetplayerInAttackRange true)
    (Utilities|FlowControl|DoOnce false
      (:Completed
        (CallFunction|StopChasingPlayer)
        (CallFunction|Attack)))
    (else
      (Variables|AI|SetplayerInAttackRange false)
      (bind _in_range_2 (CallFunction|PlayerinRange (Variables|AI|GetstopChaseDistance)))
      (if _in_range_2
        (CallFunction|ChasePlayer)
        (else
          (CallFunction|StopChasingPlayer)
          (CallFunction|AIStateMachine "NewEnumerator0")))
      (CallFunction|ResetChaseCheck))))

(event Custom|StopPatrolMovement
  (bind _waypoints (Variables|AI|GetWayPoints))
  (bind _currentwaypoint (Variables|AI|GetcurrentWayPoint))
  (bind _output (Utilities|Array|Get(acopy) _waypoints _currentwaypoint))
  ;[1 1 1] Moving to position - Since Speed = Distance / Time, Time = Distance / Speed.
  (Components|MoveComponentTo (Variables|Default|GetDefaultSceneRoot1) _output "0, 0, 0" false false (/ (Math|Vector|VectorLength (- _output (Transformation|GetActorLocation))) (Variables|Properties|GetmoveSpeed)) false) ; enters at Stop
)

(event Custom|Scan%20Player
  ;[1 1 1] Check if the player is in detect range
  (bind _in_range (CallFunction|PlayerinRange (Variables|AI|GetdetectRange)))
  (if _in_range
    (CallFunction|AIStateMachine "NewEnumerator2")
    (CallFunction|StopPatrolMovement)))

(event Custom|Reset%20Chase%20Check
  ;[1 1 1] Attack if player in attack range amd go back to patrol if player is far
  (Utilities|FlowControl|DoOnce false) ; enters at Reset
)

(event Custom|Debug
  ;[1 1 1] Debug
  (for _array_element (Variables|AI|GetWayPoints)
    (Rendering|Debug|DrawDebugSphere _array_element 3e+01 12 "(R=1.000000,G=0.770028,B=0.000000,A=1.000000)" 0.0)))

(event Custom|DealDamage
  ;[1 1 1] Damage player
  (bind _damageposition (CallFunction|DamagePosition))
  (bind (_outactors _returnvalue) (Collision|SphereOverlapActors _damageposition (Variables|Attacking|GetDamageRange) (Utilities|Array|MakeArray "ObjectTypeQuery3") 0))
  (if _returnvalue
    (for _array_element _outactors
      (Class|BPIDamageable|TakeDamage(Message) _array_element (Variables|Properties|GetdamageAmount)))))

(event Custom|Set%20Up%20Health
  ;[1 1 1] Set Up Health
  (Default|SetUp (Variables|Default|GetHealthSystem) (Variables|Properties|Gethealth))
  (CallFunction|UpdateHealthBar))

(event Custom|MoveToPosition
  ;[1 1 1] Patrol
  (if (== (Variables|AI|GetcurrentWayPoint) (- (Utilities|Array|Length (Variables|AI|GetWayPoints)) 1))
    (Variables|AI|SetcurrentWayPoint 0)
    (else
      (bind _result (Math|Integer|IncrementInt (Variables|AI|GetcurrentWayPoint))
        (:%20%20
          (Variables|AI|SetcurrentWayPoint _result)))))
  (CallFunction|Patrol))

(event Custom|Update%20HealthBar
  ;[1 1 1] Update HealthBar
  (bind _asenemy_ui (Utilities|Casting|CastToEnemy_UI (UserInterface|GetUserWidgetObject (Variables|Default|GetWidget))))
  (bind _healthpercentage (Default|GetHealthPercentage (Variables|Default|GetHealthSystem)))
  (Default|UpdateHealthUI _asenemy_ui _healthpercentage))

(event Custom|Chase%20Player
  (bind _returnvalue (Transformation|GetActorLocation))
  (bind _returnvalue_2 (Game|GetPlayerCharacter 0))
  (bind _isflying (Variables|AI|GetisFlying))
  (bind _returnvalue_3 (Transformation|GetActorLocation _returnvalue_2))
  (bind _returnvalue_4 (Math|Float|SelectFloat (.z _returnvalue_3) (.z _returnvalue) _isflying))
  (bind _returnvalue_5 (Math|Vector|MakeVector (.x _returnvalue_3) (.y _returnvalue) _returnvalue_4))
  ;[1 1 1] Chase Player
  (CallFunction|ChangeAnimation (Variables|Animation|GetWalk%20Animation))
  (CallFunction|LookatPosition _returnvalue_5)
  (Components|MoveComponentTo (Variables|Default|GetDefaultSceneRoot1) _returnvalue_5 "0, 0, 0" false false (/ (Math|Vector|VectorLength (- _returnvalue_5 (Transformation|GetActorLocation))) (Variables|Properties|GetrunSpeed)) false))

(event Custom|Damage%20Debug
  ;[1 1 1] Damage Debug
  (bind _damageposition (CallFunction|DamagePosition))
  (Rendering|Debug|DrawDebugSphere _damageposition (Variables|Attacking|GetDamageRange) 12 "(R=1.000000,G=0.000000,B=0.402194,A=1.000000)" 0.0))

(event EventBeginPlay
  (CallFunction|SetUpHealth)
  (CallFunction|AIStateMachine "NewEnumerator0"))

(event EventTick
  (params (DeltaSeconds :type Float%20%28single-precision%29))
  (if (not (Variables|Properties|GetisDead))
    (CallFunction|Debug)
    (CallFunction|AIStateMachineTick)
    (CallFunction|AttackEvent)
    (CallFunction|DamageDebug)))

(event EventTakeDamage
  (params (amount :type Integer))
  ;[1 1 1] Take Damage
  (bind _currenthealth (Default|TakeDamage (Variables|Default|GetHealthSystem) amount))
  (CallFunction|UpdateHealthBar)
  (Components|Activation|Activate (Variables|Default|GetParticleSystem) false)
  (if (<= _currenthealth 0)
    (Variables|Properties|SetisDead true)
    (CallFunction|Death)))

(fn ConstructionScript
  (for _array_element (Variables|AI|GetWayPoints)
    (Rendering|Debug|DrawDebugSphere _array_element 3e+01 12 "(R=1.000000,G=0.770028,B=0.000000,A=1.000000)" 1e+01)))

(fn PlayerinRange
  (params (Range :type Float%20%28single-precision%29))
  (return (<= (Math|Vector|Distance(Vector) (Transformation|GetActorLocation) (Transformation|GetActorLocation (Game|GetPlayerCharacter 0))) Range)))

(fn LookatPosition
  (params (Position :type Vector))
  (bind _output_get (Variables|Properties|Setscale (Transformation|GetActorScale3D)))
  (Variables|Properties|Setscale (Math|Vector|MakeVector (* (.x _output_get) -1.0) (.y _output_get) (.z _output_get)))
  (if (and (> (.x (Transformation|GetActorLocation)) (.x Position)) (not (Variables|Properties|GetisFlipped)))
    (Transformation|SetActorScale3D (Variables|Properties|Getscale))
    (Variables|Properties|SetisFlipped true)
    (elif (and (< (.x (Transformation|GetActorLocation)) (.x Position)) (Variables|Properties|GetisFlipped))
      (Transformation|SetActorScale3D (Variables|Properties|Getscale))
      (Variables|Properties|SetisFlipped false))))

(fn ChangeAnimation
  (params (New%20Animation :type Paper%20Flipbook%20Object%20Reference))
  (Sprite|SetFlipbook (Variables|Default|GetSkeleton) New%20Animation))

(fn DamagePosition
  (bind _result (Math|Float|NegateFloat (.x (Variables|Properties|Getscale)))
    (:%20%20
      (return (+ (Transformation|GetActorLocation) (Math|Vector|MakeVector (* _result (Variables|Attacking|GetAttackXOffset)) 0.0 0.0))))))