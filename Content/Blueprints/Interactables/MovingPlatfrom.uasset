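; Moving platform actor that travels continuously through an array of waypoints from BeginPlay, wrapping back to the first after the last.
; Move slides the root component to the current waypoint with MoveComponentTo, deriving duration from distance over MoveSpeed to keep the average speed consistent between legs.
; SetPosition then advances the waypoint index and calls Move again, forming an endless event-driven loop without Tick.
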(event Custom|Move
  (bind _currentwaypoint (Variables|Default|GetcurrentWayPoint))
  (bind _waypoints (Variables|Default|GetWayPoints))
  (bind _output (Utilities|Array|Get(acopy) _waypoints _currentwaypoint))
  ;[1 1 1] Moving to position - Since Speed = Distance / Time, Time = Distance / Speed.
  (Components|MoveComponentTo (Variables|Default|GetDefaultSceneRoot) _output "0, 0, 0" false false (/ (Math|Vector|VectorLength (- _output (Transformation|GetActorLocation))) (Variables|Default|GetmoveSpeed)) false)
  (CallFunction|SetPosition))

(event Custom|Set%20Position
  ;[1 1 1] Change position to go
  (if (== (Variables|Default|GetcurrentWayPoint) (- (Utilities|Array|Length (Variables|Default|GetWayPoints)) 1))
    (Variables|Default|SetcurrentWayPoint 0)
    (else
      (bind _result (Math|Integer|IncrementInt (Variables|Default|GetcurrentWayPoint))
        (:%20%20
          (Variables|Default|SetcurrentWayPoint _result)))))
  (CallFunction|Move))

(event EventBeginPlay
  (CallFunction|Move))

(event Collision|EventActorBeginOverlap
  (params (OtherActor :type Actor%20Object%20Reference)))

(event EventTick
  (params (DeltaSeconds :type Float%20%28single-precision%29)))

(fn ConstructionScript)