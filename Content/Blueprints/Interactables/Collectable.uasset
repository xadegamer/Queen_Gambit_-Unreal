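; Pickup actor that the Queen collects by touching its box, acting as either a pumpkin or a health kit depending on CollectableType.
; Pumpkins fire the OnPumpkinCollected dispatcher, while health kits heal through the Queen's HealthSystem by Amount.
; A successful pickup plays a sound, spawns a type-specific effect and destroys the actor.
; Health kits stay in the world when the Queen's health is already full.
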(event OnComponentBeginOverlap(Box)
  (params (OverlappedComponent :type Primitive%20Component%20Object%20Reference) (OtherActor :type Actor%20Object%20Reference) (OtherComp :type Primitive%20Component%20Object%20Reference) (OtherBodyIndex :type Integer) (bFromSweep :type Boolean) (SweepResult :type Hit%20Result%20Structure%20%28by%20ref%29))
  (bind _returnvalue (Transformation|GetActorLocation))
  ;[1 1 1] Collectabe colsion with player
  (bind _asqueen (Utilities|Casting|CastToQueen OtherActor))
  (switch Utilities|FlowControl|Switch|SwitchonCollectableTypes (Variables|Default|GetCollectableType)
    (:NewEnumerator0
      (Default|CallOnPumpkinCollected self)
      (Audio|PlaySound2D "/Game/Audio/DM-CGS-15.DM-CGS-15" 0.2 1.0 0.0 0 0 :!label _label)
      (switch Utilities|FlowControl|Switch|SwitchonCollectableTypes (Variables|Default|GetCollectableType)
        (:NewEnumerator0
          (Effects|SpawnEmitteratLocation "/Game/Particle/CollectPumpkinVfx.CollectPumpkinVfx" _returnvalue))
        (:NewEnumerator1
          (Effects|SpawnEmitteratLocation "/Game/Particle/CollectHealthVfx.CollectHealthVfx" _returnvalue)))
      (Actor|DestroyActor))
    (:NewEnumerator1
      (bind _not_used (CallFunction|HealthKit _asqueen))
      (if (not _not_used)
        (goto _label)))))

(event EventBeginPlay)

(event Collision|EventActorBeginOverlap
  (params (OtherActor :type Actor%20Object%20Reference)))

(event EventTick
  (params (DeltaSeconds :type Float%20%28single-precision%29)))

(fn ConstructionScript)

(fn HealthKit
  (params (player :type Queen%20Object%20Reference))
  (bind _healthsystem (Variables|/Game/Blueprints/Gameplay/Queen.Queen_C|GetHealthSystem player))
  (bind _isfull (Default|HealthFull _healthsystem))
  (if _isfull
    _
    (else
      (Default|Heal _healthsystem (Variables|Default|GetAmount))))
  (return _isfull))